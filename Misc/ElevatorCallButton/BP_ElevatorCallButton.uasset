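; Placeable elevator call button, with tinted keypad glass, that brings a nearby elevator platform to the player's height.
; Its multi-use menu hides two keypad entries and offers "Call Elevator" when activated and either unlocked or accessible.
; Calling finds the closest same-team metal track, then walks linked structures for the platform and track height limits.
; It triggers the platform's up/down use toward the player's clamped foot height, setting travel distance and a movement-check timer.
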(fn ConstructionScript
  (bind _mystaticmesh (Variables|Default|GetMyStaticMesh))
  (|CallParentFunction)
  (if (not (or (Variables|Default|GetbIsPreviewStructure) (Networking|IsDedicatedServer)))
    (bind _returnvalue (Rendering|Material|CreateDynamicMaterialInstance _mystaticmesh 1 "/Game/PrimalEarth/Structures/RemoteKeypad/Materials/RemoteKeypadGlass_MIC.RemoteKeypadGlass_MIC" :!class /Script/Engine.PrimitiveComponent))
    (Rendering|Material|SetScalarParameterValue _returnvalue "Metallic" 0.0 :!class /Script/Engine.MaterialInstanceDynamic)
    (Rendering|Material|SetScalarParameterValue _returnvalue "Roughness" 1.0 :!class /Script/Engine.MaterialInstanceDynamic)
    (Rendering|Material|SetScalarParameterValue _returnvalue "Specular" 0.0 :!class /Script/Engine.MaterialInstanceDynamic)
    (Rendering|Material|SetVectorParameterValue _returnvalue "GlassColor" "(R=0.000000,G=0.050052,B=1.000000,A=1.000000)" :!class /Script/Engine.MaterialInstanceDynamic)
    (Rendering|Material|SetMaterial _mystaticmesh 2 _returnvalue)))

(fn BPIsAllowedtoBuild
  (params (OutPlacementData :type Placement%20Data%20Structure%20%28by%20ref%29) (CurrentAllowedReason :type Integer))
  (return (Math|Integer|SelectInt 1 CurrentAllowedReason (== CurrentAllowedReason -9))))

(fn BPGetMultiUseEntries
  (params (ForPC :type Player%20Controller%20Object%20Reference) (MultiUseEntries :type Array%20of%20Multi%20Use%20Entry%20Structures))
  (bind _entriesout (CallFunction|SPUpdateMultiUseMenu ForPC MultiUseEntries self false false false false))
  (bind _entriesout_2 (CallFunction|HideKeypadMenuEntries _entriesout))
  (Utilities|FlowControl|Sequence
    (:then_0
      (bind _returnvalue (Class|PrimalStructure|AllowStructureAccess ForPC))
      (if (and (or _returnvalue (not (Variables|Default|GetbIsLocked))) (Variables|Default|GetbContainerActivated))
        (Utilities|Array|Add _entriesout_2 (Utilities|Struct|MakeMultiUseEntry "Call Elevator" 9000 99999 false))))
    (:then_1
      (return _entriesout_2))))

(fn BPTryMultiUse
  (params (ForPC :type Player%20Controller%20Object%20Reference) (UseIndex :type Integer))
  (Utilities|FlowControl|Sequence
    (:then_0
      (switch int UseIndex
        (:9000
          (CallFunction|CallElevator ForPC))))
    (:then_1
      (return false))))

(fn ReceiveBeginPlay
  (|CallParentFunction)
  (if (not (Variables|Default|GetbIsPreviewStructure))
    (Networking|SwitchHasAuthority)))

(fn CallElevator
  (params (PC :type Player%20Controller%20Object%20Reference))
  (bind _returnvalue (Pawn|GetControlledPawn PC))
  (bind (_origin _boxextent) (Collision|GetActorBounds _returnvalue true))
  (bind _elevatortrackref (CallFunction|FindClosestElevatorTrack))
  (Utilities|IsValid _elevatortrackref
    (:Is%20Valid
      (bind (_platformref _minz _maxz) (CallFunction|FindElevatorPlatform _elevatortrackref))
      (Utilities|IsValid _platformref
        (:Is%20Valid
          (Class|Actor|TryMultiUse _platformref PC (Math|Integer|SelectInt 205 206 (< (.z (Transformation|GetActorLocation _platformref)) (Math|Float|Clamp(Float) (- (.z _origin) (.z _boxextent)) _minz _maxz))))
          (Variables|/Script/ShooterGame.PrimalStructureElevatorPlatform|SetDistanceToTravel _platformref (Math|Float|Absolute(Float) (- (.z (Transformation|GetActorLocation _platformref)) (Math|Float|Clamp(Float) (- (.z _origin) (.z _boxextent)) _minz _maxz))))
          (Default|SetMovingCheckTimerEvent _platformref)
          (Class|StructuresPlus|SPMessageClient PC "Elevator Called." "Helpful"))
        (:Is%20Not%20Valid
          (Class|StructuresPlus|SPMessageClient PC "Could not find elevator platform." "Error"))))
    (:Is%20Not%20Valid
      (Class|StructuresPlus|SPMessageClient PC "Could not find elevator track." "Error"))))

(fn HideKeypadMenuEntries
  (params (EntriesIn :type Array%20of%20Multi%20Use%20Entry%20Structures))
  (for (_array_element _array_index) EntriesIn
    (if (or (== (.UseIndex (Utilities|Struct|BreakMultiUseEntry _array_element)) 700) (== (.UseIndex (Utilities|Struct|BreakMultiUseEntry _array_element)) 701))
      (LocalVariables|SetCurrentEntry_HKM _array_element)
      (Utilities|Struct|SetmembersinMultiUseEntry (LocalVariables|GetCurrentEntry_HKM) true false)
      (Utilities|Array|SetArrayElem EntriesIn _array_index (LocalVariables|GetCurrentEntry_HKM))))
  (return EntriesIn))

(fn FindClosestElevatorTrack
  (bind _returnvalue (Transformation|GetActorLocation))
  (Utilities|FlowControl|Sequence
    (:then_0
      (bind _returnvalue_2 (Class|VictoryCore|ServerOctreeOverlapActorsClass (Class|Actor|GetWorld) _returnvalue 3e+03 "STRUCTURES" "/Game/Mods/StructuresPlusMod/Misc/Elevators/Track/BP_ElevatorTrack_Metal.BP_ElevatorTrack_Metal_C" false))
      (bind _returnvalue_3 (Class|VictoryCore|SortActorsbyDistance _returnvalue _returnvalue_2))
      (bind _array_element (Utilities|Array|ForEachLoopwithBreak _returnvalue_3 :!label _label)
        (:LoopBody
          (if (== (Variables|/Script/Engine.Actor|GetTargetingTeam _array_element) (Variables|Default|GetTargetingTeam))
            (bind _asbp_elevatortrack_metal_c (Utilities|Casting|CastToBP_ElevatorTrack_Metal _array_element))
            (LocalVariables|SetretVal_FCE _asbp_elevatortrack_metal_c)
            (goto _label Break)))))
    (:then_1
      (return (LocalVariables|GetretVal_FCE)))))

(fn FindElevatorPlatform
  (params (ElevatorTrackRef :type BP%20Elevator%20Track%20Metal%20Object%20Reference))
  (LocalVariables|SetMinZ_FEP 999999999.0)
  (LocalVariables|SetMaxZ_FEP -999999999.0)
  (bind _connectedstructures (CallFunction|SPGetLinkedStructures ElevatorTrackRef true (Utilities|Array|MakeArray "/Game/Mods/StructuresPlusMod/Misc/Elevators/Platforms/Base_ElevatorPlatform.Base_ElevatorPlatform_C" "/Game/Mods/StructuresPlusMod/Misc/Elevators/Track/BP_ElevatorTrack_Metal.BP_ElevatorTrack_Metal_C") (Utilities|Array|MakeArray)))
  (for _array_element _connectedstructures
    (bind _asbase_elevatorplatform_c (Utilities|Casting|CastToBase_ElevatorPlatform _array_element)
      (:then
        (LocalVariables|SetretVal_FEP _asbase_elevatorplatform_c))
      (:CastFailed
        (bind _asbp_elevatortrack_metal_c (Utilities|Casting|CastToBP_ElevatorTrack_Metal _array_element))
        (Utilities|FlowControl|Sequence
          (:then_0
            (if (< (- (.z (.Origin (Collision|GetActorBounds _asbp_elevatortrack_metal_c true))) (.z (.BoxExtent (Collision|GetActorBounds _asbp_elevatortrack_metal_c true)))) (LocalVariables|GetMinZ_FEP))
              (LocalVariables|SetMinZ_FEP (- (.z (.Origin (Collision|GetActorBounds _asbp_elevatortrack_metal_c true))) (.z (.BoxExtent (Collision|GetActorBounds _asbp_elevatortrack_metal_c true)))))))
          (:then_1
            (if (> (+ (.z (.Origin (Collision|GetActorBounds _asbp_elevatortrack_metal_c true))) (.z (.BoxExtent (Collision|GetActorBounds _asbp_elevatortrack_metal_c true)))) (LocalVariables|GetMaxZ_FEP))
              (LocalVariables|SetMaxZ_FEP (+ (.z (.Origin (Collision|GetActorBounds _asbp_elevatortrack_metal_c true))) (.z (.BoxExtent (Collision|GetActorBounds _asbp_elevatortrack_metal_c true)))))))))))
  (return (LocalVariables|GetretVal_FEP) (LocalVariables|GetMinZ_FEP) (LocalVariables|GetMaxZ_FEP)))